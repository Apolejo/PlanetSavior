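; A human actor that wanders across the planet surface for ten seconds, then may become a city.
; A looping timer applies a small random drift and turn, re-snapping the actor to the planet's surface and normal each step.
; On expiry, a roll against BuildingPercent picks a high, medium or low population city, spawned at a random planet point rather than the human's position and attached to the planet, before the human is destroyed.
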(event Custom|DisappearHuman
  (CallFunction|BuildingChance)
  (CallFunction|SpawnBuilding)
  (Actor|DestroyActor))

(event Custom|AddVelocity
  (Transformation|AddActorLocalOffset (Variables|Default|GetStartMovement) false false)
  (Transformation|AddActorLocalRotation (Variables|Default|GetStartRotation) false false)
  (bind (_surfacelocation _surfacenormal) (Default|GetSurfaceLocationandNormalat (Variables|Default|GetPlanet_Ref) (Transformation|GetActorLocation)))
  (Transformation|SetActorLocationAndRotation _surfacelocation (Math|Rotator|MakeRotfromZX _surfacenormal (Transformation|GetActorForwardVector))))

(event EventBeginPlay
  (bind _returnvalue (Math|Random|RandomUnitVector))
  (Variables|Default|SetStartMovement (Math|Vector|MakeVector (Math|Float|Clamp(Float) (.x _returnvalue) -0.1 0.1) (Math|Float|Clamp(Float) (.y _returnvalue) -0.1 0.1) 0.0))
  (Variables|Default|SetStartRotation (Math|Rotator|MakeRotator 0.0 0.0 (Math|Float|Clamp(Float) (Math|Random|RandomFloat) -0.25 0.25)))
  (Variables|Default|SetHumanity (Math|Random|RandomInteger 15))
  (Utilities|Time|SetTimerbyEvent (delegate Custom|AddVelocity) 0.1 true)
  (Utilities|Time|SetTimerbyEvent (delegate Custom|DisappearHuman) 1e+01))

(fn ConstructionScript)

(fn BuildingChance
  (Variables|Default|SetRandom (Math|Conversions|ToFloat(Integer) (Math|Random|RandomIntegerinRange 0 100)))
  (bind (_array_element _array_index) (Utilities|Array|ForEachLoopwithBreak (Variables|Default|GetBuildingPercent) :!label _label)
    (:LoopBody
      (Variables|Default|SetProbSubstraction 1e+02)
      (if (>= (Variables|Default|GetRandom) (- (Variables|Default|GetProbSubstraction) _array_element))
        (Variables|Default|SetSetBuildingClass (+ (Math|Conversions|ToFloat(Integer) _array_index) 1.0))
        (goto _label Break)))
    (:Completed
      (return))))

(fn SpawnBuilding
  (bind _planet_ref (Variables|Default|GetPlanet_Ref))
  (bind _planet_ref_2 (Variables|Default|GetPlanet_Ref))
  (bind _planet (Variables|/Game/MotherEarth/Blueprints/Player/PlayerPlanet_Blueprint.PlayerPlanet_Blueprint_C|GetPlanet _planet_ref_2))
  (switch int (Math|Float|Truncate (Variables|Default|GetSetBuildingClass))
    (:1
      (bind _returnvalue (Utilities|SpawnLocation))
      (bind _returnvalue_2 (Game|SpawnActorfromClass "/Game/MotherEarth/Blueprints/HighPopCity_Blueprint.HighPopCity_Blueprint_C" _returnvalue "Undefined" 0 _planet_ref 0))
      (Utilities|IsValid _returnvalue_2
        (:Is%20Valid
          (Transformation|AttachComponentToComponent _returnvalue_2 _planet "None" "KeepRelative" "KeepRelative" "KeepRelative" true))))
    (:2
      (bind _returnvalue_3 (Utilities|SpawnLocation))
      (bind _returnvalue_4 (Game|SpawnActorfromClass "/Game/MotherEarth/Blueprints/MediumPopCity_Blueprint.MediumPopCity_Blueprint_C" _returnvalue_3 "Undefined" 0 _planet_ref 0))
      (Utilities|IsValid _returnvalue_4
        (:Is%20Valid
          (Transformation|AttachComponentToComponent _returnvalue_4 _planet "None" "KeepRelative" "KeepRelative" "KeepRelative" true))))
    (:3
      (bind _returnvalue_5 (Utilities|SpawnLocation))
      (bind _returnvalue_6 (Game|SpawnActorfromClass "/Game/MotherEarth/Blueprints/LowPopCity_Blueprint.LowPopCity_Blueprint_C" _returnvalue_5 "Undefined" 0 _planet_ref 0))
      (Utilities|IsValid _returnvalue_6
        (:Is%20Valid
          (Transformation|AttachComponentToComponent _returnvalue_6 _planet "None" "KeepRelative" "KeepRelative" "KeepRelative" true)))))
  (return))