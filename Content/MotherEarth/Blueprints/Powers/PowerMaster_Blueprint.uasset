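; Base Blueprint for a placeable power that periodically damages cities and reduces their population within its area.
; Until SetupMesh runs it shows a plane in place of the power mesh; placement swaps them, activates particles and destroys the actor after its lifetime.
; A looping timer started at BeginPlay drives the damage, which applies only once placed, to city actors overlapping DamageArea.
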(event Custom|SetupMesh
  (bind _powermesh (Variables|Default|GetPowerMesh))
  (bind _particlesystem (Variables|Default|GetParticleSystem))
  (Utilities|IsValid _powermesh
    (:Is%20Valid
      (Rendering|SetVisibility _powermesh true false))
    (:Is%20Not%20Valid
      _))
  (Rendering|SetVisibility (Variables|Default|GetPlane) false false)
  (Variables|Default|SetImPlaced true)
  (Utilities|IsValid _particlesystem
    (:Is%20Valid
      (Components|Activation|Activate _particlesystem false))
    (:Is%20Not%20Valid
      _))
  (Utilities|FlowControl|Delay (Variables|Default|GetLifetime))
  (CallFunction|Destroy))

(event Custom|Destroy
  (Actor|DestroyActor))

(event Custom|CauseDamage
  (if (Variables|Default|GetImPlaced)
    (for _array_element (Collision|GetOverlappingActors (Variables|Default|GetDamageArea) "/Game/MotherEarth/Blueprints/CitiesMaster_Blueprint.CitiesMaster_Blueprint_C" :!class /Script/Engine.PrimitiveComponent)
      (bind _ascities_master_blueprint (Utilities|Casting|CastToCitiesMaster_Blueprint _array_element))
      (Default|ReducePopulation _ascities_master_blueprint (Variables|Default|GetPopReduction))
      (Default|RecievingDamage _ascities_master_blueprint (Variables|Default|GetDmg)))))

(event EventBeginPlay
  (Utilities|Time|SetTimerbyEvent (EventDispatchers|CreateEvent :!event Custom|CauseDamage) (Variables|Default|GetDamageOverTime) true)
  (Rendering|SetVisibility (Variables|Default|GetPowerMesh) false false)
  (Rendering|SetVisibility (Variables|Default|GetPlane) true false))

(fn ConstructionScript)