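; Child hurricane power actor that wanders across a surface while staying aligned to it.
; On begin play, after the parent logic, a looping timer drives the movement event instead of Tick.
; Each step applies local offset and rotation from its start movement and rotation values.
; It then queries the player reference for surface location and normal, snapping position and up axis to them while keeping its forward heading.
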(event Custom|RandomMovement
  (Transformation|AddActorLocalOffset (Variables|Default|GetStartMovement) false false)
  (Transformation|AddActorLocalRotation (Variables|Default|GetStartRotation) false false)
  (bind (_surfacelocation _surfacenormal) (Default|GetSurfaceLocationandNormalat (Variables|Default|GetPlayerRef) (Transformation|GetActorLocation)))
  (Transformation|SetActorLocationAndRotation _surfacelocation (Math|Rotator|MakeRotfromZX _surfacenormal (Transformation|GetActorForwardVector))))

(event EventBeginPlay
  (|CallParentFunction)
  (Utilities|Time|SetTimerbyEvent (delegate Custom|RandomMovement) 0.1 true))

(event Collision|EventActorBeginOverlap
  (params (OtherActor :type Actor%20Object%20Reference))
  (|CallParentFunction OtherActor) ; This node is disabled and will not be called.\nDrag off pins to build functionality.
)

(event EventTick
  (params (DeltaSeconds :type Float%20%28single-precision%29))
  (|CallParentFunction DeltaSeconds) ; This node is disabled and will not be called.\nDrag off pins to build functionality.
)

(fn ConstructionScript
  (|CallParentFunction))