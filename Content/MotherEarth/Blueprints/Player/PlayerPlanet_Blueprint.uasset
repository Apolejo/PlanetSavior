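; Player planet that spins with an orbiting moon and hosts the game's civilizations, scaled to a set radius by its construction script.
; On BeginPlay it spawns random low, medium or high population cities at random surface points, oriented to the surface and attached to rotate along.
; Once the game starts, holding right mouse opens a gate for pitch-clamped spring arm camera orbiting.
; A helper projects any location onto the surface, returning point and normal.
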(event EventBeginPlay
  (bind _returnvalue (Game|GetPlayerController 0))
  (bind (_asplayer_earth_controller _bsuccess) (Utilities|Casting|CastToPlayerEarth_Controller _returnvalue))
  (if _bsuccess
    (Variables|Default|SetControllerRef _asplayer_earth_controller)
    (for _index (range 0 (Variables|Default|GetNumberOfSpawns))
      (CallFunction|SpawnCivilization))))

(event EventTick
  (params (DeltaSeconds :type Float%20%28single-precision%29))
  (Transformation|AddLocalRotation (Variables|Default|GetPlanet) "0,0.050000, 0" false false)
  (Transformation|AddWorldRotation (Variables|Default|GetMoonArm) "0.000000,0.250000, 0" false false)
  (Transformation|AddWorldRotation (Variables|Default|GetMoon) "0.000000,0.250000, 0" false false)
  (if (Variables|/Game/MotherEarth/PlayerEarth_Controller.PlayerEarth_Controller_C|GetGameStarted? (Variables|Default|GetControllerRef))
    (Utilities|FlowControl|Gate true
      (:Exit
        (CallFunction|CameraMovement)))))

(event Input|MouseEvents|RightMouseButton
  (params (Key :type Key%20Structure))
  (:Pressed
    (Utilities|FlowControl|Gate true) ; enters at Open
  )
  (:Released
    (Utilities|FlowControl|Gate true) ; enters at Close
  ))

(fn ConstructionScript
  (bind _output_get (Variables|Default|SetRadiusInUnits (* (Variables|Default|GetRadiusInMeters) 1e+02)))
  (Transformation|SetWorldScale3D (Variables|Default|GetPlanet) (Math|Conversions|ToVector(Float) (/ _output_get (.SphereRadius (Collision|GetComponentBounds (Variables|Default|GetPlanet)))))))

(fn CameraMovement
  (bind _springarm (Variables|Default|GetSpringArm))
  (bind _camera_sensitive (Variables|Default|GetCamera%20Sensitive))
  (bind _returnvalue (Transformation|GetWorldRotation _springarm))
  (Transformation|SetWorldRotation (Variables|Default|GetSpringArm) (Math|Rotator|MakeRotator (.roll _returnvalue) (Math|Float|Clamp(Float) (+ (.pitch _returnvalue) (* (Class|Actor|GetInputAxisKeyValue) _camera_sensitive)) -75.0 45.0) (+ (.yaw _returnvalue) (* (Class|Actor|GetInputAxisKeyValue) _camera_sensitive))) false false))

(fn GetSurfaceLocationandNormalat
  (params (Location :type Vector))
  (bind _returnvalue (Transformation|GetActorLocation))
  (bind _returnvalue_2 (- Location _returnvalue))
  (bind _returnvalue_3 (Math|Vector|Normalize _returnvalue_2))
  (return (+ (* _returnvalue_3 (Variables|Default|GetRadiusInUnits)) (Transformation|GetActorLocation)) _returnvalue_3))

(fn SpawnCivilization
  (bind _returnvalue (Transformation|GetActorLocation))
  (bind _output_get (Variables|Default|SetSufaceNormal (Math|Random|RandomUnitVector)))
  (switch int (Math|Random|RandomInteger 3)
    (:0
      (bind _returnvalue_2 (Game|SpawnActorfromClass "/Game/MotherEarth/Blueprints/LowPopCity_Blueprint.LowPopCity_Blueprint_C" (Math|Transform|MakeTransform (+ (* _output_get (.SphereRadius (Collision|GetComponentBounds (Variables|Default|GetPlanet)))) _returnvalue) (Math|Rotator|MakeRotator (.roll (Math|Rotator|FindLookatRotation _output_get _returnvalue)) (+ (.pitch (Math|Rotator|FindLookatRotation _output_get _returnvalue)) 9e+01) (.yaw (Math|Rotator|FindLookatRotation _output_get _returnvalue)))) "AdjustIfPossibleButDontSpawnIfColliding" 0 self 0))
      (Transformation|AttachComponentToComponent _returnvalue_2 (Variables|Default|GetPlanet) "None" "KeepRelative" "KeepRelative" "KeepRelative" true))
    (:1
      (bind _returnvalue_3 (Game|SpawnActorfromClass "/Game/MotherEarth/Blueprints/MediumPopCity_Blueprint.MediumPopCity_Blueprint_C" (Math|Transform|MakeTransform (+ (* _output_get (.SphereRadius (Collision|GetComponentBounds (Variables|Default|GetPlanet)))) _returnvalue) (Math|Rotator|MakeRotator (.roll (Math|Rotator|FindLookatRotation _output_get _returnvalue)) (+ (.pitch (Math|Rotator|FindLookatRotation _output_get _returnvalue)) 9e+01) (.yaw (Math|Rotator|FindLookatRotation _output_get _returnvalue)))) "AdjustIfPossibleButDontSpawnIfColliding" 0 self 0))
      (Transformation|AttachComponentToComponent _returnvalue_3 (Variables|Default|GetPlanet) "None" "KeepRelative" "KeepRelative" "KeepRelative" true))
    (:2
      (bind _returnvalue_4 (Game|SpawnActorfromClass "/Game/MotherEarth/Blueprints/HighPopCity_Blueprint.HighPopCity_Blueprint_C" (Math|Transform|MakeTransform (+ (* _output_get (.SphereRadius (Collision|GetComponentBounds (Variables|Default|GetPlanet)))) _returnvalue) (Math|Rotator|MakeRotator (.roll (Math|Rotator|FindLookatRotation _output_get _returnvalue)) (+ (.pitch (Math|Rotator|FindLookatRotation _output_get _returnvalue)) 9e+01) (.yaw (Math|Rotator|FindLookatRotation _output_get _returnvalue)))) "AdjustIfPossibleButDontSpawnIfColliding" 0 self 0))
      (Transformation|AttachComponentToComponent _returnvalue_4 (Variables|Default|GetPlanet) "None" "KeepRelative" "KeepRelative" "KeepRelative" true)))
  (return _returnvalue_2))