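; Master Blueprint for a destructible city on a planet, with a randomized population and a building life counter.
; MouseDamage cuts Humanity and life behind a short cooldown with a sound, while RecievingDamage subtracts a given amount of life.
; When life runs out, OnDestroy spawns tiny running humans oriented along the city's position vector, attaches them to the planet, then destroys the city.
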(event Custom|RecievingDamage
  (params (Damage :type Integer))
  (bind _output_get (Variables|Default|SetBuildingLife (- (Variables|Default|GetBuildingLife) Damage)))
  (if (<= _output_get 0)
    (CallFunction|OnDestroy)))

(event Custom|ReducePopulation
  (params (PopulationDivision :type Float%20%28single-precision%29))
  (Variables|Default|SetHumanity (Math|Float|Floor (* (Math|Conversions|ToFloat(Integer) (Variables|Default|GetHumanity)) PopulationDivision))))

(event Custom|MouseDamage
  (if (not (Variables|Default|GetClicked))
    (Variables|Default|SetClicked true)
    (Audio|PlaySound2D "/Game/MotherEarth/Music/tesla_4_corto.tesla_4_corto" 1.0 1.0 0.0 0 0)
    (CallFunction|ReducePopulation 0.75)
    (bind _output_get (Variables|Default|SetBuildingLife (- (Variables|Default|GetBuildingLife) 1)))
    (if (<= _output_get 0)
      (CallFunction|OnDestroy)
      (else
        (Utilities|FlowControl|Delay 0.5)
        (Variables|Default|SetClicked false)))))

(event EventBeginPlay
  (Variables|Default|SetMaxHumans (Math|Random|RandomInteger (Variables|Default|GetMaxRandomHumans)))
  (Variables|Default|SetHumanity (Math|Random|RandomInteger (Variables|Default|GetMaxHumanity))))

(fn ConstructionScript)

(fn OnDestroy
  (bind _returnvalue (Transformation|GetActorLocation))
  (bind _planet_ref (Variables|Default|GetPlanet_Ref))
  (for _index (range 0 (Variables|Default|GetMaxHumans))
    (bind _returnvalue_2 (Game|SpawnActorfromClass "/Game/MotherEarth/Blueprints/RunningHumans_Blueprint.RunningHumans_Blueprint_C" (Math|Transform|MakeTransform (+ (* "0, 0, 0" (.SphereRadius (Collision|GetComponentBounds (Variables|/Game/MotherEarth/Blueprints/Player/PlayerPlanet_Blueprint.PlayerPlanet_Blueprint_C|GetPlanet _planet_ref)))) _returnvalue) (Math|Rotator|MakeRotfromZ _returnvalue) "0.010000,0.010000,0.010000") "Undefined" 0 _planet_ref 0))
    (Transformation|AttachComponentToComponent _returnvalue_2 (Variables|/Game/MotherEarth/Blueprints/Player/PlayerPlanet_Blueprint.PlayerPlanet_Blueprint_C|GetPlanet (Variables|Default|GetPlanet_Ref)) "None" "KeepWorld" "KeepRelative" "KeepRelative" true))
  (Actor|DestroyActor))